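; Interactable actor that glows when the cursor hovers over it or something overlaps its box, printing debug text for these events.
; ActivateGlow sets the "Selected" material scalar on all its static mesh components.
; Hover and standing flags gate switch-off, but the check needs both true right after clearing one, so the glow never turns off.
; Its InteractionComp Interact event only prints the interacting actor's name.
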(event `self.StaticMeshComponent.OnBeginCursorOver`
  (params (TouchedComponent :type "PrimitiveComponent Object Reference"))
  (`self.ActivateGlow` true :!label _label)
  (`KismetSystemLibrary.PrintText` "Cursor Over")
  (set `self.IsHover` true))

(event `self.Box.OnBeginCursorOver`
  (params (TouchedComponent :type "PrimitiveComponent Object Reference"))
  (goto _label))

(event `self.Box.OnEndCursorOver`
  (params (TouchedComponent :type "PrimitiveComponent Object Reference"))
  (set `self.IsHover` false :!label _label_2)
  (if (not (`KismetMathLibrary.BooleanNAND` (`self.IsStanding`) (`self.IsHover`)))
    (`self.ActivateGlow` false)))

(event `self.StaticMeshComponent.OnEndCursorOver`
  (params (TouchedComponent :type "PrimitiveComponent Object Reference"))
  (goto _label_2))

(event `self.Box.OnComponentBeginOverlap`
  (params (OverlappedComponent :type "PrimitiveComponent Object Reference") (OtherActor :type "Actor Object Reference") (OtherComp :type "PrimitiveComponent Object Reference") (OtherBodyIndex :type Integer) (bFromSweep :type Boolean) (SweepResult :type "HitResult Structure (by ref)"))
  (`self.ActivateGlow` true)
  (`KismetSystemLibrary.PrintText` "Actor Walk")
  (set `self.IsStanding` true))

(event `self.Box.OnComponentEndOverlap`
  (params (OverlappedComponent :type "PrimitiveComponent Object Reference") (OtherActor :type "Actor Object Reference") (OtherComp :type "PrimitiveComponent Object Reference") (OtherBodyIndex :type Integer))
  (set `self.IsStanding` false)
  (if (not (`KismetMathLibrary.BooleanNAND` (`self.IsStanding`) (`self.IsHover`)))
    (`self.ActivateGlow` false)))

(event `self.InteractionComp.Interact`
  (params (`Interacting Actor` :type "Actor Object Reference"))
  (`KismetSystemLibrary.PrintText` (`KismetTextLibrary.Conv_StringToText` (`KismetSystemLibrary.GetObjectName` `Interacting Actor`))))

(fn `ActivateGlow`
  (params (isActive :type Boolean))
  (locals (NewLocalVar_0 :type "Float (double-precision)"))
  (for _array_element (`self.K2_GetComponentsByClass` "/Script/Engine.StaticMeshComponent")
    (if isActive
      (`MeshComponent.SetScalarParameterValueOnMaterials` _array_element "Selected" 1.0)
      (else
        (`MeshComponent.SetScalarParameterValueOnMaterials` _array_element "Selected" 0.0)))))

(fn `UserConstructionScript`)